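; BP_Ennemi_Voleur is an enemy that repeatedly fires BP_Ennemi_Voleur_Tir projectiles, with selectable behaviours: look at player, rotation, translation, both, or immobile.
; While Actif, Tick runs the enabled modes, using a detection sphere for actors tagged "Voleur" and timelines for spinning or spline ping-pong.
; All modes share one DoOnce-gated shot, reset after a reload delay and not gated by detection.
; Désactivation pauses the behaviour logic until a timeline finishes.
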(event OnComponentBeginOverlap(Sphere)
  (params (OverlappedComponent :type Primitive%20Component%20Object%20Reference) (OtherActor :type Actor%20Object%20Reference) (OtherComp :type Primitive%20Component%20Object%20Reference) (OtherBodyIndex :type Integer) (bFromSweep :type Boolean) (SweepResult :type Hit%20Result%20Structure%20%28by%20ref%29))
  ;[1 1 1 0.5] Mode de tir de l'ennemi
  ;;[1 0 0] Mode de Fonctionnement : Regarde le joueur
  ;;;[1 1 1] Portée de détection de l'ennemi
  (Utilities|IsValid OtherActor
    (:Is%20Valid
      (if (Actor|ActorHasTag OtherActor "Voleur")
        (Variables|Default|SetVoleur_a_Portée true)))))

(event OnComponentEndOverlap(Sphere)
  (params (OverlappedComponent :type Primitive%20Component%20Object%20Reference) (OtherActor :type Actor%20Object%20Reference) (OtherComp :type Primitive%20Component%20Object%20Reference) (OtherBodyIndex :type Integer))
  ;[1 1 1 0.5] Mode de tir de l'ennemi
  ;;[1 0 0] Mode de Fonctionnement : Regarde le joueur
  ;;;[1 1 1] Portée de détection de l'ennemi
  (Utilities|IsValid OtherActor
    (:Is%20Valid
      (if (Actor|ActorHasTag OtherActor "Voleur")
        (Variables|Default|SetVoleur_a_Portée false)))))

(event Custom|Désactivation
  ;[1 1 1] Désactivation de l'ennemi
  (Variables|Default|SetActif%20? false)
  (Timeline|Durée%20Désactivation PlayFromStart
    (:Finished
      (Variables|Default|SetActif%20? true))))

(event Custom|Tir%20des%20autres%20mode%20de%20Fonctionnement
  (bind _skeletalmesh (Variables|Default|GetSkeletalMesh))
  ;[1 1 1 0.5] Mode de tir de l'ennemi
  ;;[0 1 1] Mode de Fonctionnement : Immobile
  (Utilities|FlowControl|DoOnce false :!label _label
    (:Completed
      (bind _returnvalue (Game|SpawnActorfromClass "/Game/Maps/Partie/Ennemi/BP_Ennemi_Voleur_Tir.BP_Ennemi_Voleur_Tir_C" (Math|Transform|MakeTransform (+ (Transformation|GetWorldLocation _skeletalmesh) "") (Transformation|GetWorldRotation _skeletalmesh) "1.000000,1.000000,1.000000") "Undefined" "MultiplyWithRoot" 0 0))
      (Utilities|IsValid _returnvalue
        (:Is%20Valid
          (Game|Components|ProjectileMovement|SetVelocityinLocalSpace (Variables|/Game/Maps/Partie/Ennemi/BP_Ennemi_Voleur_Tir.BP_Ennemi_Voleur_Tir_C|GetProjectileMovement _returnvalue) (* (Math|Vector|GetForwardVector "0.000000,180.000000,0.000000") (Variables|Default|GetPuissance%20du%20tir)))
          (Utilities|FlowControl|Delay (Variables|Default|GetTemps%20de%20recharge%20du%20tir))
          (goto _label Reset))))))

(event EventTick
  (params (DeltaSeconds :type Float%20%28single-precision%29))
  (bind _skeletalmesh (Variables|Default|GetSkeletalMesh))
  (bind _skeletalmesh_2 (Variables|Default|GetSkeletalMesh))
  (bind _spline (Variables|Default|GetSpline))
  (bind _spline_2 (Variables|Default|GetSpline))
  (bind _skeletalmesh_3 (Variables|Default|GetSkeletalMesh))
  (bind _skeletalmesh_4 (Variables|Default|GetSkeletalMesh))
  ;[1 1 1 0.5] Mode de tir de l'ennemi
  ;;[1 1 1] L'ennemi est actif ?
  (if (Variables|Default|GetActif%20?)
    (Utilities|FlowControl|Sequence
      (:then_0
        ;;[1 1 1] Mode de Fonctionnement de l'ennemi
        (if (Variables|Default|GetMode%20de%20Fonctionnement%20:%20Regarde%20le%20joueur)
          ;;[1 0 0] Mode de Fonctionnement : Regarde le joueur
          (Utilities|FlowControl|Sequence
            (:then_0
              ;;;[1 1 1] Se tourne vers le voleur
              (if (Variables|Default|GetVoleur_a_Portée)
                (bind _outactors (Actor|GetAllActorswithTag "Voleur"))
                (for _array_element _outactors
                  (Transformation|SetActorRotation (Math|Rotator|FindLookatRotation (Transformation|GetActorLocation _array_element) (Transformation|GetActorLocation))))))
            (:then_1
              (CallFunction|TirDesAutresModeDeFonctionnement)))))
      (:then_1
        (if (Variables|Default|GetMode%20de%20Fonctionnement%20:%20Rotation%20+%20Translation)
          ;;[1 0.3 0] Mode de Fonctionnement : Rotation + Translation
          (Utilities|FlowControl|Sequence
            (:then_0
              (Utilities|FlowControl|DoOnce false
                (:Completed
                  (Components|Timeline|SetPlayRate (Variables|Default|GetTimeline_Rotation%20+%20Translation_Partie_Translation) (/ 1.0 (Variables|Default|GetDurée%20Translation)))
                  (bind _newtrack_0 (Timeline|Timeline_Rotation%20+%20Translation_Partie_Translation PlayFromStart)
                    (:Update
                      (Transformation|SetWorldLocation _skeletalmesh_4 (Spline|GetLocationatDistanceAlongSpline _spline_2 (* _newtrack_0 (Spline|GetSplineLength _spline_2)) "World") false false)
                      ;;;[1 1 1] Ajustement de la rotation
                      (Transformation|AddRelativeRotation _skeletalmesh_4 (Variables|Default|GetAjustement%20Rotation) false false)
                      (Utilities|FlowControl|DoOnce false
                        (:Completed
                          (Components|Timeline|SetPlayRate (Variables|Default|GetTimeline_Rotation%20+%20Translation_Partie_Rotation) (/ 1.0 (Variables|Default|GetDurée%20Rotation)))
                          (bind _newtrack_0_2 (Timeline|Timeline_Rotation%20+%20Translation_Partie_Rotation PlayFromStart)
                            (:Update
                              (Transformation|SetWorldRotation (Variables|Default|GetSkeletalMesh) (Math|Rotator|MakeRotator 0.0 0.0 (* _newtrack_0_2 3.6e+02)) false false))
                            (:Finished
                              (Utilities|FlowControl|Delay 0.0)
                              (Timeline|Timeline_Rotation%20+%20Translation_Partie_Rotation PlayFromStart))))))
                    (:Finished
                      (Utilities|FlowControl|FlipFlop
                        (:A
                          (Timeline|Timeline_Rotation%20+%20Translation_Partie_Translation Reverse))
                        (:B
                          (Timeline|Timeline_Rotation%20+%20Translation_Partie_Translation PlayFromStart))))))))
            (:then_1
              (CallFunction|TirDesAutresModeDeFonctionnement)))))
      (:then_2
        (if (Variables|Default|GetMode%20de%20Fonctionnement%20:%20Rotation)
          ;;[1 1 0] Mode de Fonctionnement : Rotation
          (Utilities|FlowControl|Sequence
            (:then_0
              (Utilities|FlowControl|DoOnce false
                (:Completed
                  (Components|Timeline|SetPlayRate (Variables|Default|GetTimeline_Rotation) (/ 1.0 (Variables|Default|GetDurée%20Rotation)))
                  (bind _newtrack_0_3 (Timeline|Timeline_Rotation PlayFromStart)
                    (:Update
                      (Transformation|SetWorldRotation _skeletalmesh_3 (Math|Rotator|MakeRotator 0.0 0.0 (* _newtrack_0_3 3.6e+02)) false false)
                      ;;;[1 1 1] Si le static mesh se s'aligne pas bien
                      (Transformation|AddRelativeRotation _skeletalmesh_3 (Variables|Default|GetAjustement%20Rotation) false false))
                    (:Finished
                      (Utilities|FlowControl|Delay 0.0)
                      (Timeline|Timeline_Rotation PlayFromStart))))))
            (:then_1
              (CallFunction|TirDesAutresModeDeFonctionnement)))))
      (:then_3
        (if (Variables|Default|GetMode%20de%20Fonctionnement%20:%20Translation)
          ;;[0 1 0] Mode de Fonctionnement : Translation
          (Utilities|FlowControl|Sequence
            (:then_0
              (Utilities|FlowControl|DoOnce false
                (:Completed
                  (Components|Timeline|SetPlayRate (Variables|Default|GetTimeline_Translation) (/ 1.0 (Variables|Default|GetDurée%20Translation)))
                  (bind _newtrack_0_4 (Timeline|Timeline_Translation PlayFromStart)
                    (:Update
                      (Transformation|SetWorldLocation _skeletalmesh_2 (Spline|GetLocationatDistanceAlongSpline _spline (* _newtrack_0_4 (Spline|GetSplineLength _spline)) "World") false false)
                      ;;;[1 1 1] Si le static mesh se s'aligne pas bien
                      (Transformation|AddRelativeRotation _skeletalmesh_2 (Variables|Default|GetAjustement%20Rotation) false false))
                    (:Finished
                      (Utilities|FlowControl|FlipFlop
                        (:A
                          (Timeline|Timeline_Translation Reverse))
                        (:B
                          (Timeline|Timeline_Translation PlayFromStart))))))))
            (:then_1
              (CallFunction|TirDesAutresModeDeFonctionnement)))))
      (:then_4
        (if (Variables|Default|GetMode%20de%20Fonctionnement%20:%20Immobile)
          ;;[0 1 1] Mode de Fonctionnement : Immobile
          (Utilities|FlowControl|DoOnce false :!label _label
            (:Completed
              (bind _returnvalue (Game|SpawnActorfromClass "/Game/Maps/Partie/Ennemi/BP_Ennemi_Voleur_Tir.BP_Ennemi_Voleur_Tir_C" (Math|Transform|MakeTransform (+ (Transformation|GetWorldLocation _skeletalmesh) "") (Transformation|GetWorldRotation _skeletalmesh) "1.000000,1.000000,1.000000") "Undefined" "MultiplyWithRoot" 0 0))
              (Utilities|IsValid _returnvalue
                (:Is%20Valid
                  (Game|Components|ProjectileMovement|SetVelocityinLocalSpace (Variables|/Game/Maps/Partie/Ennemi/BP_Ennemi_Voleur_Tir.BP_Ennemi_Voleur_Tir_C|GetProjectileMovement _returnvalue) (* (Math|Vector|GetForwardVector "0.000000,180.000000,0.000000") (Variables|Default|GetPuissance%20du%20tir)))
                  (Utilities|FlowControl|Delay (Variables|Default|GetTemps%20de%20recharge%20du%20tir))
                  (goto _label Reset))))))))))

(fn ConstructionScript)