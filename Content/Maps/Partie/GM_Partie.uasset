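; GM_Partie is the match game mode that spawns the Voleur (thief) character and drives its aim toward the mouse cursor.
; BeginPlay triggers BP_Spawn_Voleur's coordinate retrieval, and PositionSpawnVoleur spawns and possesses the thief, adds the input mapping and shows UI_Voleur outside N_Niveau_1.
; Each Tick traces from the cursor into the world, ignoring "Mur"-tagged walls cached once, and passes the impact point to the thief's rotation function.
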(event Custom|Position%20Spawn%20Voleur
  (params (Coordonnées%20Spawn%20Voleur :type Vector))
  (bind _returnvalue (Game|GetPlayerController 0))
  ;[1 1 1] Création des personnages Guerrier/Mage/Voleur
  (bind _returnvalue_2 (Game|SpawnActorfromClass "/Game/Maps/Partie/Personnages-Joueur/Personnage_Voleur/BP_Personnage_Voleur.BP_Personnage_Voleur_C" (Math|Transform|MakeTransform Coordonnées%20Spawn%20Voleur "0, 0, 0" "1.000000,1.000000,1.000000") "Undefined" "MultiplyWithRoot" 0 0))
  ;[1 1 1] Prise de contrôle du Guerrier au début de la partie
  (bind _aspc_partie (Utilities|Casting|CastToPC_Partie _returnvalue)
    (:then
      (Pawn|Possess _aspc_partie _returnvalue_2)
      (Utilities|IsValid _aspc_partie
        (:Is%20Valid
          (Input|AddMappingContext (PlayerController|LocalPlayerSubsystems|GetEnhancedInputLocalPlayerSubsystem _returnvalue) "/Game/Maps/Partie/Personnages-Joueur/Input/IMC_Default.IMC_Default" 0 "(bIgnoreAllPressedKeysUntilRelease=True,bForceImmediately=False,bNotifyUserSettings=False)")
          (bind _returnvalue_3 (Game|GetCurrentLevelName true))
          (if (not (Utilities|Enum|Equal(Enum) _returnvalue_3 "N_Niveau_1"))
            (bind _returnvalue_4 (UserInterface|CreateWidget "/Game/Maps/Partie/Personnages-Joueur/Personnage_Voleur/UI_Voleur.UI_Voleur_C"))
            (bind _output_get (Variables|Default|SetUI_Voleur _returnvalue_4))
            (UserInterface|Viewport|AddtoViewport _output_get 0)))))
    (:CastFailed
      (Development|PrintString "Hello"))))

(event EventBeginPlay
  (Utilities|FlowControl|Sequence
    (:then_0
      (bind _returnvalue (Actor|GetActorOfClass "/Game/Maps/Partie/Personnages-Joueur/Personnage_Voleur/BP_Spawn_Voleur.BP_Spawn_Voleur_C"))
      (Default|RécupérationCoordonées _returnvalue))))

(event EventTick
  (params (DeltaSeconds :type Float%20%28single-precision%29))
  (bind _returnvalue (Game|GetPlayerController 0))
  (bind _newvar (Variables|Default|GetNewVar))
  (bind (_locationx _locationy) (Game|Player|GetMousePosition _returnvalue))
  (bind (_worldlocation _worlddirection) (Class|PlayerController|DeprojectScreenPositiontoWorld _returnvalue _locationx _locationy))
  ;[1 1 1] Position du curseur dans le monde. Puis Rotation des personnages par rapport à ce point
  (Utilities|FlowControl|Sequence
    (:then_0
      (Utilities|FlowControl|DoOnce false
        (:Completed
          (bind _outactors (Actor|GetAllActorswithTag "Mur"))
          (for _array_element _outactors
            (Utilities|Array|AddUnique _newvar _array_element)))))
    (:then_1
      (bind _outhit (Collision|LineTraceByChannel _worldlocation (+ _worldlocation (* _worlddirection 1e+04)) "TraceTypeQuery1" false _newvar "None"))
      (Utilities|FlowControl|Sequence
        (:then_0
          (bind _returnvalue_2 (Actor|GetActorOfClass "/Game/Maps/Partie/Personnages-Joueur/Personnage_Voleur/BP_Personnage_Voleur.BP_Personnage_Voleur_C"))
          (Utilities|IsValid _returnvalue_2
            (:Is%20Valid
              (Default|RotationDuPersonnage _returnvalue_2 (.ImpactPoint (Collision|BreakHitResult _outhit))))))))))

(fn ConstructionScript)