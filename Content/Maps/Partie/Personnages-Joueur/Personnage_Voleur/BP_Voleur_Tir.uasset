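; Shot actor for the thief (Voleur) player character that deactivates enemies and triggers buttons on contact.
; A Box begin-overlap checks component tags: "Ennemi" calls Désactivation on the owning BP_Ennemi_Voleur, and "Bouton" calls EffetDuBouton on the owning BP_Interaction_Bouton_Voleur.
; Otherwise, overlapping an actor tagged "Niveau" destroys the shot, which is the only case where this graph destroys it.
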(event OnComponentBeginOverlap(Box)
  (params (OverlappedComponent :type Primitive%20Component%20Object%20Reference) (OtherActor :type Actor%20Object%20Reference) (OtherComp :type Primitive%20Component%20Object%20Reference) (OtherBodyIndex :type Integer) (bFromSweep :type Boolean) (SweepResult :type Hit%20Result%20Structure%20%28by%20ref%29))
  (bind _returnvalue (Components|GetOwner OtherComp))
  (if (Components|ComponentHasTag OtherComp "Ennemi")
    (bind _asbp_ennemi_voleur (Utilities|Casting|CastToBP_Ennemi_Voleur _returnvalue))
    (Default|Désactivation _asbp_ennemi_voleur)
    (elif (Components|ComponentHasTag OtherComp "Bouton")
      (bind _asbp_interaction_bouton_voleur (Utilities|Casting|CastToBP_Interaction_Bouton_Voleur _returnvalue))
      (Default|EffetDuBouton _asbp_interaction_bouton_voleur)
      (elif (Actor|ActorHasTag OtherActor "Niveau")
        (Actor|DestroyActor)))))

(fn ConstructionScript)