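; Interactive door that slides a cube along a spline when the Effetdelaporte event receives its door number.
; The first trigger plays a timeline scaled by the door's duration, mapping its value to spline distance while keeping the actor's rotation.
; Later triggers reverse it only for plate-activated doors.
; A FlipFlop on timeline completion alternates between optional delayed closing and clearing the activated flag if reactivation is allowed.
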(event Custom|Effet%20de%20la%20porte
  (params (N°%20de%20porte :type Integer))
  (bind _spline (Variables|Default|GetSpline))
  ;[1 1 1] N° de la porte à activer
  (if (== N°%20de%20porte (Variables|Default|GetN°%20de%20la%20porte))
    ;[1 1 1] Si n'est pas activé, elle s'active
    (if (Variables|Default|GetActivé)
      (if (Variables|Default|GetActivation%20par%20plaque)
        ;[1 1 1] Ouverture en X secondes ("Durée") selon une spline
        (bind _newtrack_0 (Timeline|Timeline Reverse)
          (:Update
            (Transformation|SetWorldLocationAndRotation (Variables|Default|GetCube) (Spline|GetLocationatDistanceAlongSpline _spline (* _newtrack_0 (Spline|GetSplineLength _spline)) "World") (Transformation|GetActorRotation) false false))
          (:Finished
            ;[1 1 1] Si elle peut se refermer, elle se referme au bout de X secondes
            (Utilities|FlowControl|FlipFlop
              (:A
                (if (Variables|Default|GetPeut%20se%20refermé%20?)
                  (Utilities|FlowControl|Delay (Math|Conversions|ToFloat(Integer) (Variables|Default|GetPeut%20se%20refermé%20en%20_%20secondes)))
                  (Timeline|Timeline Reverse)))
              (:B
                ;[1 1 1] Peut-être contrôlé par un interrupteur ?
                (if (Variables|Default|GetPeut-être%20réactivé%20?)
                  (Variables|Default|SetPeut-être%20réactivé%20? true)
                  (Variables|Default|SetActivé false)))))))
      (else
        (Variables|Default|SetActivé true)
        (Components|Timeline|SetPlayRate (Variables|Default|GetTimeline) (/ 1.0 (Variables|Default|GetDurée)))
        (Timeline|Timeline PlayFromStart)))))

(fn ConstructionScript)