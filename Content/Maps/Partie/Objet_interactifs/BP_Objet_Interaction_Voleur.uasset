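; BP_Objet_Interaction_Voleur is an interactive object for the thief (Voleur) character.
; When an actor tagged "Voleur" enters its sphere, it looks up BP_Personnage_Voleur by class and registers itself as an available interaction.
; When that actor leaves, it tells the thief to reset its interactable objects in range.
; Its effect event only prints an activation message.
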(event OnComponentBeginOverlap(Sphere)
  (params (OverlappedComponent :type Primitive%20Component%20Object%20Reference) (OtherActor :type Actor%20Object%20Reference) (OtherComp :type Primitive%20Component%20Object%20Reference) (OtherBodyIndex :type Integer) (bFromSweep :type Boolean) (SweepResult :type Hit%20Result%20Structure%20%28by%20ref%29))
  (if (Actor|ActorHasTag OtherActor "Voleur")
    (bind _returnvalue (Actor|GetActorOfClass "/Game/Maps/Partie/Personnages-Joueur/Personnage_Voleur/BP_Personnage_Voleur.BP_Personnage_Voleur_C"))
    (Default|InteractionAvecUnObjetPossible _returnvalue self)))

(event OnComponentEndOverlap(Sphere)
  (params (OverlappedComponent :type Primitive%20Component%20Object%20Reference) (OtherActor :type Actor%20Object%20Reference) (OtherComp :type Primitive%20Component%20Object%20Reference) (OtherBodyIndex :type Integer))
  (if (Actor|ActorHasTag OtherActor "Voleur")
    (bind _returnvalue (Actor|GetActorOfClass "/Game/Maps/Partie/Personnages-Joueur/Personnage_Voleur/BP_Personnage_Voleur.BP_Personnage_Voleur_C"))
    (Default|RéinitialisationDesObjetsInteractifsÀPortée _returnvalue)))

(event Custom|Effet%20de%20l'objet
  (Development|PrintString "Activé !"))

(fn ConstructionScript)