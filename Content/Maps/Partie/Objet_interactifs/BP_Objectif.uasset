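; BP_Objectif is a numbered, moving objective that wins the game when an actor tagged "Voleur" reaches it.
; A start event, meant to match its number, plays a Timeline moving the Cube along a Spline by distance, setting world rotation from the spline's local rotation.
; Events switch between normal, accelerated and decelerated durations, applied as play rate on each update.
; Overlapping the Sphere with that tag opens the N_Démarrage level.
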(event OnComponentBeginOverlap(Sphere)
  (params (OverlappedComponent :type Primitive%20Component%20Object%20Reference) (OtherActor :type Actor%20Object%20Reference) (OtherComp :type Primitive%20Component%20Object%20Reference) (OtherBodyIndex :type Integer) (bFromSweep :type Boolean) (SweepResult :type Hit%20Result%20Structure%20%28by%20ref%29))
  ;[1 1 1] Lorsque le joueur atteint l'objectif, il gagne la partie
  (if (Actor|ActorHasTag OtherActor "Voleur")
    (Game|OpenLevel(byObjectReference) "/Game/Maps/Démarrage/N_Démarrage.N_Démarrage")))

(event Custom|Décélération
  ;[1 1 1] Modification de la vitesse de l'objectif
  (Variables|Default|SetDurée%20Actuelle (Variables|Default|GetDurée%20Décélérée)))

(event Custom|Vitesse%20normale
  ;[1 1 1] Modification de la vitesse de l'objectif
  (Variables|Default|SetDurée%20Actuelle (Variables|Default|GetDurée%20Normale)))

(event Custom|Accélération
  ;[1 1 1] Modification de la vitesse de l'objectif
  (Variables|Default|SetDurée%20Actuelle (Variables|Default|GetDurée%20Accélérée)))

(event Custom|Départ%20de%20l'objectif
  (params (N°%20de%20l'objectif :type Integer))
  (bind _timeline (Variables|Default|GetTimeline))
  (bind _spline (Variables|Default|GetSpline))
  ;[1 1 1] L'objectif N°x part
  (if (== N°%20de%20l'objectif (Variables|Default|GetN°%20de%20l'objectif))
    ;[1 1 1] En vitesse de base
    (Variables|Default|SetDurée%20Actuelle (Variables|Default|GetDurée%20Normale))
    ;[1 1 1] Déplacement et rotation selon une spline (en tenant compte de sa vitesse actuelle
    (Components|Timeline|SetPlayRate _timeline (/ 1.0 (Variables|Default|GetDurée%20Actuelle)))
    (bind _newtrack_0 (Timeline|Timeline PlayFromStart)
      (:Update
        (Components|Timeline|SetPlayRate _timeline (/ 1.0 (Variables|Default|GetDurée%20Actuelle)))
        (Transformation|SetWorldLocationAndRotation (Variables|Default|GetCube) (Spline|GetLocationatDistanceAlongSpline _spline (* _newtrack_0 (Spline|GetSplineLength _spline)) "World") (Spline|GetRotationatDistanceAlongSpline _spline (* _newtrack_0 (Spline|GetSplineLength _spline)) "Local") false false)))))

(fn ConstructionScript)