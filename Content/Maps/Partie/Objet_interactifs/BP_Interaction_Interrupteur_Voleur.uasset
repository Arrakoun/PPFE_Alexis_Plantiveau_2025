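; Thief-only switch that plays an activation sound and triggers doors or lights, either once or as a toggle.
; Sphere overlap with the "Voleur"-tagged actor registers it with BP_Personnage_Voleur and shows an "E" prompt.
; Effetdel'objet broadcasts an ID number to every BP_Porte or BP_Lumière, based on behaviour booleans, and swaps on/off lever meshes.
; Single-use modes remove prompt and sphere; toggles use DoOnce with a 0.2s reset to flip once per loop.
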(event OnComponentBeginOverlap(Sphere)
  (params (OverlappedComponent :type Primitive%20Component%20Object%20Reference) (OtherActor :type Actor%20Object%20Reference) (OtherComp :type Primitive%20Component%20Object%20Reference) (OtherBodyIndex :type Integer) (bFromSweep :type Boolean) (SweepResult :type Hit%20Result%20Structure%20%28by%20ref%29))
  ;[1 1 1] Visibilité de la possibilité d'intéraction (Image "E")
  (Utilities|IsValid OtherActor
    (:Is%20Valid
      (if (Actor|ActorHasTag OtherActor "Voleur")
        (bind _returnvalue (Actor|GetActorOfClass "/Game/Maps/Partie/Personnages-Joueur/Personnage_Voleur/BP_Personnage_Voleur.BP_Personnage_Voleur_C"))
        (Default|InteractionAvecUnObjetPossible _returnvalue self)
        (CallFunction|RendreLeWidget"E"Visible)))))

(event OnComponentEndOverlap(Sphere)
  (params (OverlappedComponent :type Primitive%20Component%20Object%20Reference) (OtherActor :type Actor%20Object%20Reference) (OtherComp :type Primitive%20Component%20Object%20Reference) (OtherBodyIndex :type Integer))
  ;[1 1 1] Visibilité de la possibilité d'intéraction (Image "E")
  (Utilities|IsValid OtherActor
    (:Is%20Valid
      (if (Actor|ActorHasTag OtherActor "Voleur")
        (bind _returnvalue (Actor|GetActorOfClass "/Game/Maps/Partie/Personnages-Joueur/Personnage_Voleur/BP_Personnage_Voleur.BP_Personnage_Voleur_C"))
        (Default|RéinitialisationDesObjetsInteractifsÀPortée _returnvalue)
        (CallFunction|RendreLeWidget"E"Invisible)))))

(event Custom|Effet%20de%20l'objet
  (bind _embout_activé (Variables|Default|GetEmbout_activé))
  (bind _embout_activé_2 (Variables|Default|GetEmbout_activé))
  (bind _widget (Variables|Default|GetWidget))
  (Audio|Components|Audio|Play (Variables|Default|GetA_Activation) 0.0)
  ;[1 0 0] Comportement : Porte - Activation unique
  (if (Variables|Default|GetComportement%20:%20Porte%20-%20Activation%20Unique)
    (Utilities|FlowControl|DoOnce false
      (:Completed
        (bind _outactors (Actor|GetAllActorsOfClass "/Game/Maps/Partie/Objet_interactifs/BP_Porte.BP_Porte_C"))
        (for _array_element _outactors
          (Default|EffetDeLaPorte _array_element (Variables|Default|GetN°de%20la%20porte))
          (Rendering|SetVisibility (Variables|Default|GetEmbout_activé) true false)
          (Rendering|SetVisibility (Variables|Default|GetBaton_désactivé) false false)
          (Utilities|IsValid (Variables|Default|GetSphere)
            (:Is%20Valid
              (Utilities|IsValid _widget
                (:Is%20Valid
                  (Components|DestroyComponent _widget))))))))
    (else
      ;[0 0 1] Comportement : Porte - Activation / Désactivation
      (if (Variables|Default|GetComportement%20:%20Porte%20-%20Activation%20/%20Désactivation)
        (bind _outactors_2 (Actor|GetAllActorsOfClass "/Game/Maps/Partie/Objet_interactifs/BP_Porte.BP_Porte_C"))
        (for _array_element_2 _outactors_2
          (Default|EffetDeLaPorte _array_element_2 (Variables|Default|GetN°de%20la%20porte))
          (Utilities|FlowControl|DoOnce false :!label _label
            (:Completed
              (Utilities|FlowControl|FlipFlop
                (:A
                  (Rendering|SetVisibility _embout_activé_2 true false)
                  (Rendering|SetVisibility (Variables|Default|GetBaton_désactivé) false false))
                (:B
                  (Rendering|SetVisibility _embout_activé_2 false false)
                  (Rendering|SetVisibility (Variables|Default|GetEmbout_désactivé) true false)))
              (Utilities|FlowControl|DoOnce false :!label _label_2
                (:Completed
                  (Utilities|FlowControl|Delay 0.2)
                  (Utilities|FlowControl|Sequence
                    (:then_0
                      (goto _label Reset))
                    (:then_1
                      (goto _label_2 Reset))))))))
        (else
          ;[1 1 0] Comportement : Lumière - Activation unique
          (if (Variables|Default|GetComportement%20:%20Lumière%20-%20Activation%20Unique)
            (Utilities|FlowControl|DoOnce false
              (:Completed
                (bind _outactors_3 (Actor|GetAllActorsOfClass "/Game/Projet/Actors/Environnement/BP_Lumière.BP_Lumière_C"))
                (for _array_element_3 _outactors_3
                  (Default|ModificationDeLaLumière _array_element_3 (Variables|Default|GetN°%20de%20la%20lumière))
                  (Rendering|SetVisibility (Variables|Default|GetEmbout_activé) true false)
                  (Rendering|SetVisibility (Variables|Default|GetBaton_désactivé) false false)
                  (Components|DestroyComponent (Variables|Default|GetWidget)))))
            (else
              ;[0 0 1] Comportement : Lumière - Activation / Désactivation
              (if (Variables|Default|GetComportement%20:%20Lumière%20-%20Activation%20Désactivation)
                (bind _outactors_4 (Actor|GetAllActorsOfClass "/Game/Projet/Actors/Environnement/BP_Lumière.BP_Lumière_C"))
                (for _array_element_4 _outactors_4
                  (Default|ModificationDeLaLumière _array_element_4 (Variables|Default|GetN°%20de%20la%20lumière))
                  (Utilities|FlowControl|DoOnce false :!label _label_3
                    (:Completed
                      (Utilities|FlowControl|FlipFlop
                        (:A
                          (Rendering|SetVisibility _embout_activé true false)
                          (Rendering|SetVisibility (Variables|Default|GetBaton_désactivé) false false))
                        (:B
                          (Rendering|SetVisibility _embout_activé false false)
                          (Rendering|SetVisibility (Variables|Default|GetEmbout_désactivé) true false)))
                      (Utilities|FlowControl|DoOnce false :!label _label_4
                        (:Completed
                          (Utilities|FlowControl|Delay 0.2)
                          (Utilities|FlowControl|Sequence
                            (:then_0
                              (goto _label_3 Reset))
                            (:then_1
                              (goto _label_4 Reset))))))))))))))))

(event Custom|Rendre%20le%20widget%20"E"%20invisible
  (bind _widget (Variables|Default|GetWidget))
  ;[1 1 1] Réglage de départ : Baton_activé, Embout_activé et Widget "E" caché + Quand rendre le widget "E" visible ou non
  (Utilities|IsValid _widget
    (:Is%20Valid
      (Rendering|SetVisibility _widget false false))))

(event Custom|Rendre%20le%20widget%20"E"%20visible
  (bind _widget (Variables|Default|GetWidget))
  ;[1 1 1] Réglage de départ : Baton_activé, Embout_activé et Widget "E" caché + Quand rendre le widget "E" visible ou non
  (Utilities|IsValid _widget
    (:Is%20Valid
      (Rendering|SetVisibility _widget true false))))

(event EventBeginPlay
  (bind _widget (Variables|Default|GetWidget))
  ;[1 1 1] Réglage de départ : Baton_activé, Embout_activé et Widget "E" caché + Quand rendre le widget "E" visible ou non
  (Rendering|SetVisibility (Variables|Default|GetEmbout_activé) false false)
  (Utilities|IsValid _widget
    (:Is%20Valid
      (Rendering|SetVisibility _widget false false))))

(fn ConstructionScript)