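; BP_Plaque_porte is an interactive plate that triggers doors when an actor tagged "Voleur" (the thief player) enters its collision box.
; The overlap fires only once, activating N1 to N4, playing torch and activation audio, and switching the plane's emissive material parameter to its activated value.
; It then calls EffetDeLaPorte on every BP_Porte in the level, passing the plate's door number to identify the linked door.
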(event OnComponentBeginOverlap(Box)
  (params (OverlappedComponent :type Primitive%20Component%20Object%20Reference) (OtherActor :type Actor%20Object%20Reference) (OtherComp :type Primitive%20Component%20Object%20Reference) (OtherBodyIndex :type Integer) (bFromSweep :type Boolean) (SweepResult :type Hit%20Result%20Structure%20%28by%20ref%29))
  ;[1 1 1] Lorsque le joueur "Voleur' entre dans la box de collision, l'objectif lié à ce BP par la variable "N° de l'objectif à faire partir" commence son déplacement
  (if (Actor|ActorHasTag OtherActor "Voleur")
    (Utilities|FlowControl|DoOnce false
      (:Completed
        (Components|Activation|SetActive (Variables|Default|GetN_4) true false)
        (Audio|Components|Audio|Play (Variables|Default|GetA_Torche) 0.0)
        (Audio|Components|Audio|Play (Variables|Default|GetA_Activation) 0.5)
        (Rendering|Material|SetScalarParameterValueonMaterials (Variables|Default|GetPlane) "Émissive activé / désactivé" (Variables|Default|GetÉmissive%20lorsque%20activé))
        (bind _outactors (Actor|GetAllActorsOfClass "/Game/Maps/Partie/Objet_interactifs/BP_Porte.BP_Porte_C"))
        (for _array_element _outactors
          (Default|EffetDeLaPorte _array_element (Variables|Default|GetN°%20de%20la%20porte)))))))

(fn ConstructionScript)