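; BP_Emplacement is a board slot actor with a type identifying it as a player or opponent slot, persistent or not.
; BeginPlay branches on that type, but every branch is still empty.
; A Box collision detects actors tagged as the cursor: entry has no effect yet, while exit only prints a debug message.
; A Widget is present but unused, so the slot is currently a skeleton.
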(event OnComponentBeginOverlap(Box)
  (params (OverlappedComponent :type Primitive%20Component%20Object%20Reference) (OtherActor :type Actor%20Object%20Reference) (OtherComp :type Primitive%20Component%20Object%20Reference) (OtherBodyIndex :type Integer) (bFromSweep :type Boolean) (SweepResult :type Hit%20Result%20Structure%20%28by%20ref%29))
  (if (Actor|ActorHasTag OtherActor "Curseur")
    _))

(event OnComponentEndOverlap(Box)
  (params (OverlappedComponent :type Primitive%20Component%20Object%20Reference) (OtherActor :type Actor%20Object%20Reference) (OtherComp :type Primitive%20Component%20Object%20Reference) (OtherBodyIndex :type Integer))
  (if (Actor|ActorHasTag OtherActor "Curseur")
    (Development|PrintString "Sorti")))

(event EventBeginPlay
  (if (not (== (Variables|Default|GetType%20d'emplacement) "Persistant-Joueur"))
    (if (not (== (Variables|Default|GetType%20d'emplacement) "Persistant-Adversaire"))
      (if (not (== (Variables|Default|GetType%20d'emplacement) "Adversaire"))
        (if (== (Variables|Default|GetType%20d'emplacement) "Joueur")
          _)))))

(fn ConstructionScript)