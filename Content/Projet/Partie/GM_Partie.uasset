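; Match game mode that spawns the player's character and turns characters toward the mouse cursor.
; BeginPlay requests coordinates from the Voleur spawn point; the Guerrier and Mage requests are disconnected.
; Spawn events create each class, but only the Voleur is possessed, given input mapping and a HUD.
; Tick traces under the cursor, ignoring "Mur"-tagged actors cached once, and passes the impact point to each class's rotation function.
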(event Custom|Position%20Spawn%20Voleur
  (params (Coordonnées%20Spawn%20Voleur :type Vector))
  ;[1 1 1] Création des personnages Guerrier/Mage/Voleur
  (bind _returnvalue (Game|SpawnActorfromClass "/Game/Projet/Actors/Personnages-Joueur/Personnage_Voleur/BP_Personnage_Voleur.BP_Personnage_Voleur_C" (Math|Transform|MakeTransform Coordonnées%20Spawn%20Voleur "0, 0, 0" "1.000000,1.000000,1.000000") "Undefined" "MultiplyWithRoot" 0 0))
  ;[1 1 1] Prise de contrôle du Guerrier au début de la partie
  (bind _aspc_partie (Utilities|Casting|CastToPC_Partie (Game|GetPlayerController 0)))
  (Pawn|Possess _aspc_partie _returnvalue)
  (Utilities|IsValid (PlayerController|LocalPlayerSubsystems|GetEnhancedInputLocalPlayerSubsystem _aspc_partie)
    (:Is%20Valid
      (Input|AddMappingContext (PlayerController|LocalPlayerSubsystems|GetEnhancedInputLocalPlayerSubsystem _aspc_partie) "/Game/Projet/Actors/Personnages-Joueur/Input/IMC_Default.IMC_Default" 0 "(bIgnoreAllPressedKeysUntilRelease=True,bForceImmediately=False,bNotifyUserSettings=False)")
      (bind _returnvalue_2 (UserInterface|CreateWidget "/Game/Projet/Actors/Personnages-Joueur/Personnage_Voleur/UI_Voleur.UI_Voleur_C"))
      (bind _output_get (Variables|Default|SetUI_Voleur _returnvalue_2))
      (UserInterface|Viewport|AddtoViewport _output_get 0))))

(event Custom|Position%20Spawn%20Guerrier
  (params (Coordonnées%20Spawn%20Guerrier :type Vector))
  ;[1 1 1] Création des personnages Guerrier/Mage/Voleur
  (Game|SpawnActorfromClass "/Game/Projet/Actors/Personnages-Joueur/Personnage_Guerrier/BP_Personnage_Guerrier.BP_Personnage_Guerrier_C" (Math|Transform|MakeTransform Coordonnées%20Spawn%20Guerrier "0, 0, 0" "1.000000,1.000000,1.000000") "Undefined" "MultiplyWithRoot" 0 0))

(event Custom|Position%20Spawn%20Mage
  (params (Coordonnées%20Spawn%20Mage :type Vector))
  ;[1 1 1] Création des personnages Guerrier/Mage/Voleur
  (Game|SpawnActorfromClass "/Game/Projet/Actors/Personnages-Joueur/Personnage_Mage/BP_Personnage_Mage.BP_Personnage_Mage_C" (Math|Transform|MakeTransform Coordonnées%20Spawn%20Mage "0, 0, 0" "1.000000,1.000000,1.000000") "Undefined" "MultiplyWithRoot" 0 0))

(event EventBeginPlay
  (Utilities|FlowControl|Sequence
    (:then_0
      (bind _returnvalue (Actor|GetActorOfClass "/Game/Projet/Actors/Personnages-Joueur/Personnage_Voleur/BP_Spawn_Voleur.BP_Spawn_Voleur_C"))
      (Default|RécupérationCoordonées _returnvalue))))

(event EventTick
  (params (DeltaSeconds :type Float%20%28single-precision%29))
  (bind _returnvalue (Game|GetPlayerController 0))
  (bind _newvar (Variables|Default|GetNewVar))
  (bind (_locationx _locationy) (Game|Player|GetMousePosition _returnvalue))
  (bind (_worldlocation _worlddirection) (Class|PlayerController|DeprojectScreenPositiontoWorld _returnvalue _locationx _locationy))
  ;[1 1 1] Position du curseur dans le monde. Puis Rotation des personnages par rapport à ce point
  (Utilities|FlowControl|Sequence
    (:then_0
      (Utilities|FlowControl|DoOnce false
        (:Completed
          (bind _outactors (Actor|GetAllActorswithTag "Mur"))
          (for _array_element _outactors
            (Utilities|Array|AddUnique _newvar _array_element)))))
    (:then_1
      (bind _outhit (Collision|LineTraceByChannel _worldlocation (+ _worldlocation (* _worlddirection 1e+04)) "TraceTypeQuery1" false _newvar "None"))
      (Utilities|FlowControl|Sequence
        (:then_0
          (bind _returnvalue_2 (Actor|GetActorOfClass "/Game/Projet/Actors/Personnages-Joueur/Personnage_Guerrier/BP_Personnage_Guerrier.BP_Personnage_Guerrier_C"))
          (Utilities|IsValid _returnvalue_2
            (:Is%20Valid
              (Default|RotationDuPersonnage _returnvalue_2 (.ImpactPoint (Collision|BreakHitResult _outhit))))))
        (:then_1
          (bind _returnvalue_3 (Actor|GetActorOfClass "/Game/Projet/Actors/Personnages-Joueur/Personnage_Mage/BP_Personnage_Mage.BP_Personnage_Mage_C"))
          (Utilities|IsValid _returnvalue_3
            (:Is%20Valid
              (Default|RotationDuPersonnage _returnvalue_3 (.ImpactPoint (Collision|BreakHitResult _outhit))))))
        (:then_2
          (bind _returnvalue_4 (Actor|GetActorOfClass "/Game/Projet/Actors/Personnages-Joueur/Personnage_Voleur/BP_Personnage_Voleur.BP_Personnage_Voleur_C"))
          (Utilities|IsValid _returnvalue_4
            (:Is%20Valid
              (Default|RotationDuPersonnage _returnvalue_4 (.ImpactPoint (Collision|BreakHitResult _outhit))))))))))

(fn ConstructionScript)