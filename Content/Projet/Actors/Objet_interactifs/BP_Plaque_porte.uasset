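; BP_Plaque_porte is an interactive trigger plate that lets the thief player (tag "Voleur") set linked doors in motion.
; When a tagged actor enters or leaves its collision Box, it gets every BP_Porte in the level and calls EffetDeLaPorte with its NDeLaPorte number.
; Enter and exit send the identical call, so matching the number and choosing the movement are left to BP_Porte.
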(event OnComponentBeginOverlap(Box)
  (params (OverlappedComponent :type Primitive%20Component%20Object%20Reference) (OtherActor :type Actor%20Object%20Reference) (OtherComp :type Primitive%20Component%20Object%20Reference) (OtherBodyIndex :type Integer) (bFromSweep :type Boolean) (SweepResult :type Hit%20Result%20Structure%20%28by%20ref%29))
  ;[1 1 1] Lorsque le joueur "Voleur' entre dans la box de collision, l'objectif lié à ce BP par la variable "N° de l'objectif à faire partir" commence son déplacement
  (if (Actor|ActorHasTag OtherActor "Voleur")
    (bind _outactors (Actor|GetAllActorsOfClass "/Game/Projet/Actors/Objet_interactifs/BP_Porte.BP_Porte_C"))
    (for _array_element _outactors
      (Default|EffetDeLaPorte _array_element (Variables|Default|GetN°%20de%20la%20porte)))))

(event OnComponentEndOverlap(Box)
  (params (OverlappedComponent :type Primitive%20Component%20Object%20Reference) (OtherActor :type Actor%20Object%20Reference) (OtherComp :type Primitive%20Component%20Object%20Reference) (OtherBodyIndex :type Integer))
  ;[1 1 1] Lorsque le joueur "Voleur' entre dans la box de collision, l'objectif lié à ce BP par la variable "N° de l'objectif à faire partir" commence son déplacement
  (if (Actor|ActorHasTag OtherActor "Voleur")
    (bind _outactors (Actor|GetAllActorsOfClass "/Game/Projet/Actors/Objet_interactifs/BP_Porte.BP_Porte_C"))
    (for _array_element _outactors
      (Default|EffetDeLaPorte _array_element (Variables|Default|GetN°%20de%20la%20porte)))))

(fn ConstructionScript)