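; BP_Interaction_Bouton_Voleur is an interactive button, named for the thief (Voleur), that triggers doors or lights.
; Its Effetdubouton event checks two flags, with the door option taking priority over the light option.
; It broadcasts a door or light number to every BP_Porte or BP_Lumière actor found with GetAllActorsOfClass, calling EffetDeLaPorte or ModificationDeLaLumière on each.
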(event Custom|Effet%20du%20bouton
  (if (Variables|Default|GetOuvre%20une%20porte)
    (bind _outactors (Actor|GetAllActorsOfClass "/Game/Projet/Actors/Objet_interactifs/BP_Porte.BP_Porte_C"))
    (for _array_element _outactors
      (Default|EffetDeLaPorte _array_element (Variables|Default|GetN°de%20la%20porte)))
    (elif (Variables|Default|GetÉteint/Allume%20une%20lumière)
      (bind _outactors_2 (Actor|GetAllActorsOfClass "/Game/Projet/Actors/Environnement/BP_Lumière.BP_Lumière_C"))
      (for _array_element_2 _outactors_2
        (Default|ModificationDeLaLumière _array_element_2 (Variables|Default|GetN°%20de%20la%20lumière))))))

(fn ConstructionScript)