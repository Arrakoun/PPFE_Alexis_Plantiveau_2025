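; Interactive door that opens and closes along a spline when the Effetdelaporte event carries its door number.
; Boolean flags pick one of four behaviors: plate-driven, one-shot, toggle, or timed auto-close.
; Each has its own Timeline, rate-scaled by the open/close duration, moving Parents along the spline with the actor's rotation.
; Timed mode calls its Delay-then-reverse from Timeline Update and re-arms on every second Finished.
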(event Custom|Effet%20de%20la%20porte
  (params (N°%20de%20porte :type Integer))
  (bind _spline (Variables|Default|GetSpline))
  (bind _spline_2 (Variables|Default|GetSpline))
  (bind _spline_3 (Variables|Default|GetSpline))
  (bind _spline_4 (Variables|Default|GetSpline))
  ;[1 1 1] N° de la porte à activer
  (if (== N°%20de%20porte (Variables|Default|GetN°%20de%20la%20porte))
    ;[1 1 1] Activation par plaque ?
    (if (Variables|Default|GetComportement%20:%20Activation%20par%20plaque)
      ;[1 0 0] Comportement : Activation par plaque
      (Utilities|FlowControl|FlipFlop
        (:A
          ;;[1 1 1] Ouverture en X secondes ("Durée") selon une spline
          (Components|Timeline|SetPlayRate (Variables|Default|GetTimeline_0) (/ 1.0 (Variables|Default|GetDurée%20Ouverture%20/%20Fermeture)))
          (bind _newtrack_0 (Timeline|Timeline_0 Play)
            (:Update
              (Transformation|SetWorldLocationAndRotation (Variables|Default|GetParents) (Spline|GetLocationatDistanceAlongSpline _spline_2 (* _newtrack_0 (Spline|GetSplineLength _spline_2)) "World") (Transformation|GetActorRotation) false false))))
        (:B
          (Timeline|Timeline_0 Reverse)))
      (else
        ;[1 1 1] Activation par plaque ?
        (if (Variables|Default|GetComportement%20:%20Activation%20unique)
          ;[1 1 0] Comportement : Activation unique
          (Utilities|FlowControl|DoOnce false
            (:Completed
              ;;[1 1 1] Ouverture en X secondes ("Durée") selon une spline
              (Components|Timeline|SetPlayRate (Variables|Default|GetTimeline_1) (/ 1.0 (Variables|Default|GetDurée%20Ouverture%20/%20Fermeture)))
              (bind _newtrack_0_2 (Timeline|Timeline_1 Play)
                (:Update
                  (Transformation|SetWorldLocationAndRotation (Variables|Default|GetParents) (Spline|GetLocationatDistanceAlongSpline _spline_4 (* _newtrack_0_2 (Spline|GetSplineLength _spline_4)) "World") (Transformation|GetActorRotation) false false)))))
          (else
            ;[1 1 1] Activation par plaque ?
            (if (Variables|Default|GetComportement%20:%20Activation%20/%20Desactivation)
              ;[0 1 0] Comportement : Activation / Désactivation
              (Utilities|FlowControl|FlipFlop
                (:A
                  ;;[1 1 1] Ouverture en X secondes ("Durée") selon une spline
                  (Components|Timeline|SetPlayRate (Variables|Default|GetTimeline_2) (/ 1.0 (Variables|Default|GetDurée%20Ouverture%20/%20Fermeture)))
                  (bind _newtrack_0_3 (Timeline|Timeline_2 Play)
                    (:Update
                      (Transformation|SetWorldLocationAndRotation (Variables|Default|GetParents) (Spline|GetLocationatDistanceAlongSpline _spline (* _newtrack_0_3 (Spline|GetSplineLength _spline)) "World") (Transformation|GetActorRotation) false false))))
                (:B
                  (Timeline|Timeline_2 Reverse)))
              (else
                ;[1 1 1] Activation par plaque ?
                (if (Variables|Default|GetComportement%20:%20Activation%20Chronométré)
                  ;[0 0 1] Comportement : Activation Chronométré
                  (Utilities|FlowControl|DoOnce false :!label _label
                    (:Completed
                      ;;[1 1 1] Ouverture en X secondes ("Durée") selon une spline
                      (Components|Timeline|SetPlayRate (Variables|Default|GetTimeline_3) (/ 1.0 (Variables|Default|GetDurée%20Ouverture%20/%20Fermeture)))
                      (bind _newtrack_0_4 (Timeline|Timeline_3 Play)
                        (:Update
                          (Transformation|SetWorldLocationAndRotation (Variables|Default|GetParents) (Spline|GetLocationatDistanceAlongSpline _spline_3 (* _newtrack_0_4 (Spline|GetSplineLength _spline_3)) "World") (Transformation|GetActorRotation) false false)
                          (Utilities|FlowControl|Delay (Variables|Default|GetComportement%20:%20Activatin%20Chronométré%20-%20Durée%20Activé))
                          (Timeline|Timeline_3 Reverse))
                        (:Finished
                          (Utilities|FlowControl|FlipFlop
                            (:B
                              (goto _label Reset))))))))))))))))

(fn ConstructionScript)