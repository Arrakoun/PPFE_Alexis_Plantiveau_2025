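; Light actor that, while lit, changes the speed of BP_Objectif when a "Voleur"-tagged actor enters its sphere: red (malus) accelerates it, green decelerates it.
; Leaving the sphere of a lit light restores normal speed.
; An ID-based event triggers the light with once, toggle or timed behavior, flipping either on/off or malus/bonus.
; The construction script previews the initial color and off state on the SpotLight.
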(event OnComponentBeginOverlap(Sphere)
  (params (OverlappedComponent :type Primitive%20Component%20Object%20Reference) (OtherActor :type Actor%20Object%20Reference) (OtherComp :type Primitive%20Component%20Object%20Reference) (OtherBodyIndex :type Integer) (bFromSweep :type Boolean) (SweepResult :type Hit%20Result%20Structure%20%28by%20ref%29))
  ;[1 1 1] Effet de la lumière
  (Utilities|IsValid OtherActor
    (:Is%20Valid
      (if (Actor|ActorHasTag OtherActor "Voleur")
        (if (not (Variables|Default|GetÉtat%20:%20Éteinte%20?))
          (bind _returnvalue (Actor|GetActorOfClass "/Game/Projet/Actors/Objet_interactifs/BP_Objectif.BP_Objectif_C"))
          (if (Variables|Default|GetÉtat%20:%20Malus%20?)
            (Default|Accélération _returnvalue)
            (else
              (Default|Décélération _returnvalue))))))))

(event OnComponentEndOverlap(Sphere)
  (params (OverlappedComponent :type Primitive%20Component%20Object%20Reference) (OtherActor :type Actor%20Object%20Reference) (OtherComp :type Primitive%20Component%20Object%20Reference) (OtherBodyIndex :type Integer))
  ;[1 1 1] Effet de la lumière
  (Utilities|IsValid OtherActor
    (:Is%20Valid
      (if (Actor|ActorHasTag OtherActor "Voleur")
        (if (not (Variables|Default|GetÉtat%20:%20Éteinte%20?))
          (bind _returnvalue (Actor|GetActorOfClass "/Game/Projet/Actors/Objet_interactifs/BP_Objectif.BP_Objectif_C"))
          (Default|VitesseNormale _returnvalue))))))

(event Custom|Modification%20de%20la%20lumière
  (params (N°%20de%20la%20lumière :type Integer))
  ;[1 1 1] Identification de la lumière
  (if (== N°%20de%20la%20lumière (Variables|Default|GetN°%20de%20la%20lumière))
    ;[1 1 1] Comportement d'activation
    (if (Variables|Default|GetComportement%20:%20Activation%20unique)
      (Utilities|FlowControl|DoOnce false
        (:Completed
          (CallFunction|ApplicationDeL'effet)))
      (elif (Variables|Default|GetComportement%20:%20Activation%20/%20Désactivation)
        (CallFunction|ApplicationDeL'effet)
        (elif (Variables|Default|GetComportement%20:%20Activation%20Chronométré)
          (CallFunction|ApplicationDeL'effet)
          (Utilities|FlowControl|Delay (Variables|Default|GetComportement%20:%20Activation%20Chronométré%20-%20Durée))
          (CallFunction|ApplicationDeL'effet))))))

(event Custom|Type%20d'effet%20:%20Malus%20-%20Bonus
  ;[1 1 0] Type d'effet : Malus / Bonus
  (if (Variables|Default|GetÉtat%20:%20Malus%20?)
    (Rendering|Components|Light|SetLightColor (Variables|Default|GetSpotLight) "(R=0.000000,G=1.000000,B=0.000000,A=1.000000)" true)
    (Variables|Default|SetÉtat%20:%20Malus%20? false)
    (else
      (Rendering|Components|Light|SetLightColor (Variables|Default|GetSpotLight) "(R=1.000000,G=0.000000,B=0.000000,A=1.000000)" true)
      (Variables|Default|SetÉtat%20:%20Malus%20? true))))

(event Custom|Type%20d'effet%20:%20Activation%20-%20Désactivation
  ;[1 0 0] Type d'effet : allumé / éteint
  (if (Variables|Default|GetÉtat%20:%20Éteinte%20?)
    (Variables|Default|SetÉtat%20:%20Éteinte%20? false)
    (Rendering|Components|Light|SetIntensity (Variables|Default|GetSpotLight) 8e+06)
    (else
      (Variables|Default|SetÉtat%20:%20Éteinte%20? true)
      (Rendering|Components|Light|SetIntensity (Variables|Default|GetSpotLight) 0.0))))

(event Custom|Application%20de%20l'effet
  ;[1 1 1] Application de l'effet
  (if (Variables|Default|GetType%20d'effet%20:%20Activation%20/%20Désactivation)
    (CallFunction|TypeD'effet:Activation-Désactivation)
    (elif (Variables|Default|GetType%20d'effet%20:%20Malus%20/%20Bonus)
      (CallFunction|TypeD'effet:Malus-Bonus))))

(fn ConstructionScript
  (if (Variables|Default|GetÉtat%20:%20Malus%20?)
    (Rendering|Components|Light|SetLightColor (Variables|Default|GetSpotLight) "(R=1.000000,G=0.000000,B=0.000000,A=1.000000)" true)
    (else
      (Rendering|Components|Light|SetLightColor (Variables|Default|GetSpotLight) "(R=0.000000,G=1.000000,B=0.000000,A=1.000000)" true)))
  (if (Variables|Default|GetÉtat%20:%20Éteinte%20?)
    (Rendering|Components|Light|SetIntensity (Variables|Default|GetSpotLight) 0.0)))