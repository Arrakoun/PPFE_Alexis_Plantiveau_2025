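; Game mode for a match that spawns the cursor and player, then tracks the mouse's position in the world.
; BeginPlay stores BP_curseur, has player controller 0 possess a new BP_Joueur, and adds the IMC_Joueur input context.
; Tick deprojects the mouse into a Visibility trace, skipping "Ignore"-tagged actors gathered once.
; The impact point is saved to CoordonnéesDeLaSouris and passed to SetActorLocation, which has no explicit Curseur target.
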(event EventBeginPlay
  (bind _returnvalue (Game|GetPlayerController 0))
  (bind _returnvalue_2 (PlayerController|LocalPlayerSubsystems|GetEnhancedInputLocalPlayerSubsystem _returnvalue))
  ;[1 1 1] Création du curseur
  (bind _returnvalue_3 (Game|SpawnActorfromClass "/Game/Curseur/BP_curseur.BP_curseur_C" (Math|Transform|MakeTransform "0, 0, 0" "0, 0, 0" "1.000000,1.000000,1.000000") "Undefined" "MultiplyWithRoot" 0 0))
  (Variables|Default|SetCurseur _returnvalue_3)
  (bind _returnvalue_4 (Game|SpawnActorfromClass "/Game/BP_Joueur.BP_Joueur_C" (Math|Transform|MakeTransform "0.000000,0.000000,300.000000" "0, 0, 0" "1.000000,1.000000,1.000000") "Undefined" "MultiplyWithRoot" 0 0))
  (Pawn|Possess _returnvalue _returnvalue_4)
  (Utilities|IsValid _returnvalue_2
    (:Is%20Valid
      (Input|AddMappingContext _returnvalue_2 "/Game/Inputs/IMC_Joueur.IMC_Joueur" 0 "(bIgnoreAllPressedKeysUntilRelease=True,bForceImmediately=False,bNotifyUserSettings=False)"))))

(event EventTick
  (params (DeltaSeconds :type Float%20%28single-precision%29))
  (bind _returnvalue (Game|GetPlayerController 0))
  (bind _newvar (Variables|Default|GetNewVar))
  (bind (_locationx _locationy) (Game|Player|GetMousePosition _returnvalue))
  (bind (_worldlocation _worlddirection) (Class|PlayerController|DeprojectScreenPositiontoWorld _returnvalue _locationx _locationy))
  ;[1 1 1] Position du curseur dans le monde.
  (Utilities|FlowControl|Sequence
    (:then_0
      (Utilities|FlowControl|DoOnce false
        (:Completed
          (bind _outactors (Actor|GetAllActorswithTag "Ignore"))
          (for _array_element _outactors
            (Utilities|Array|AddUnique _newvar _array_element)))))
    (:then_1
      (bind _outhit (Collision|LineTraceByChannel _worldlocation (+ _worldlocation (* _worlddirection 1e+04)) "TraceTypeQuery1" false _newvar "None"))
      (bind _output_get (Variables|Default|SetCoordonnées%20de%20la%20souris (.ImpactPoint (Collision|BreakHitResult _outhit))))
      (Transformation|SetActorLocation _output_get false false))))

(fn ConstructionScript)